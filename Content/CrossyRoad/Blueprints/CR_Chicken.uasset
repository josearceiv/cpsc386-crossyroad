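; CR_Chicken is the first-person player character for a Crossy Road-style game, tracking a count of lanes crossed.
; Axis inputs drive camera look and camera-relative movement, while Jump also plays a hop sound, located at the camera's forward vector rather than its position.
; Tick disables input whenever IsAlive is false.
; AddLaneCrossedPoint increments the score, which resets on BeginPlay; Drown is an empty stub.
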(event EventBeginPlay
  (Variables|Default|SetlanesCrossedPoints 0))

(event EventTick
  (params (DeltaSeconds :type Float%20%28single-precision%29))
  (if (not (Variables|Default|GetisAlive))
    (Input|DisableInput 0)))

(event Input|ActionEvents|InputActionJump
  (params (Key :type Key%20Structure :default "None"))
  (:Pressed
    ;[1 1 1] Jumping
    (Character|Jump)
    (Audio|PlaySoundatLocation "/Game/CrossyRoad/Audio/Player_Actor/hop2b.hop2b" (Math|Vector|GetForwardVector (Variables|Default|GetFirst_Person_Camera)) "0, 0, 0" 1.0 1.0 0.0 0 0 0))
  (:Released
    (Character|StopJumping)))

(event Input|AxisEvents|InputAxisMoveFoward
  (params (AxisValue :type Float%20%28single-precision%29))
  ;[1 1 1] Basic Movement
  (Pawn|Input|AddMovementInput (Math|Vector|GetForwardVector (Variables|Default|GetFirst_Person_Camera)) AxisValue false))

(event Input|AxisEvents|InputAxisTurn
  (params (AxisValue :type Float%20%28single-precision%29))
  ;[1 1 1] Camera Movement
  (Pawn|Input|AddControllerYawInput AxisValue))

(event Input|AxisEvents|InputAxisLookUp
  (params (AxisValue :type Float%20%28single-precision%29))
  ;[1 1 1] Camera Movement
  (Pawn|Input|AddControllerPitchInput AxisValue))

(event Input|AxisEvents|InputAxisMoveRight
  (params (AxisValue :type Float%20%28single-precision%29))
  (Pawn|Input|AddMovementInput (Math|Vector|GetRightVector (Variables|Default|GetFirst_Person_Camera)) AxisValue false))

(fn ConstructionScript)

(fn AddLaneCrossedPoint
  (Variables|Default|SetlanesCrossedPoints (+ (Variables|Default|GetlanesCrossedPoints) 1)))

(fn GetLaneCrossedPoints
  (CallFunction|GetLaneCrossedPoints)
  (return))

(fn Drown)